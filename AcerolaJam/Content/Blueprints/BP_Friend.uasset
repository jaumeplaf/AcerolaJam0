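; BP_Friend is a collectible companion that the player finds by touching it and that then follows the player.
; The first overlap with its Interact sphere fires the Found event with effects and sound, then removes the sphere and starts a self-restarting AIMoveTo loop.
; A looping timer writes its position to MPC_Player per FriendTag for materials to read.
; BeginPlay randomizes its material hue and binds BP_MapManager state events, whose handlers are empty.
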(event `self.ReceiveBeginPlay`
  (bind _outactors (`GameplayStatics.GetAllActorsOfClass` "/Game/Blueprints/BP_MapManager.BP_MapManager_C"))
  (bind _output (`|GetArrayItem` _outactors))
  (add `/Game/Blueprints/BP_MapManager.Map_Initial` _output (`|CreateDelegate` :!event `Initial`))
  (add `/Game/Blueprints/BP_MapManager.Map_Initial` _output (`|CreateDelegate` :!event `Initial`))
  (add `/Game/Blueprints/BP_MapManager.Map_Corrupted` _output (`|CreateDelegate` :!event `Corrupted`))
  (add `/Game/Blueprints/BP_MapManager.Map_Final` _output (`|CreateDelegate` :!event `Final`))
  (add `self.Found` (`|CreateDelegate` :!event `FriendFound`))
  (bind _returnvalue (`KismetMaterialLibrary.CreateDynamicMaterialInstance` (`PrimitiveComponent.GetMaterial` (`self.Mesh`) 1)))
  (`PrimitiveComponent.SetMaterial` (`self.Mesh`) 1 _returnvalue)
  (`MaterialInstanceDynamic.SetScalarParameterValue` _returnvalue "HueShift" (`KismetMathLibrary.RandomFloat`))
  (`KismetSystemLibrary.K2_ClearAndInvalidateTimerHandle` (stale `FriendFound` _returnvalue)))

(event `Initial`)

(event `self.Interact.OnComponentBeginOverlap`
  (params (OverlappedComponent :type "PrimitiveComponent Object Reference") (OtherActor :type "Actor Object Reference") (OtherComp :type "PrimitiveComponent Object Reference") (OtherBodyIndex :type Integer) (bFromSweep :type Boolean) (SweepResult :type "HitResult Structure (by ref)"))
  (bind _mesh (`self.Mesh`))
  (if (not (`self.isFound`))
    (`self.Found`)
    (set `self.isFound` true)
    (`NiagaraFunctionLibrary.SpawnSystemAttached` "/Game/VFX/FX_Found.FX_Found" _mesh "None" (`SceneComponent.K2_GetComponentLocation` _mesh) (struct) "KeepWorldPosition" true)
    (switch `int` (`KismetMathLibrary.RandomInteger` 1)
      (:`0`
        (`GameplayStatics.SpawnSound2D` "/Game/Audio/AUD_Found01.AUD_Found01" 1.0 1.0 0.0 null))
      (:`1`
        (`GameplayStatics.SpawnSound2D` "/Game/Audio/AUD_Found02.AUD_Found02" 1.0 1.0 0.0 null)))
    (`KismetSystemLibrary.Delay` 0.2)
    (`GameplayStatics.GetActorOfClass` null)))

(event `Corrupted`)

(event `Final`)

(event `self.ReceiveTick`
  (params (DeltaSeconds :type "Float (single-precision)")))

(event `self.Interact.OnComponentEndOverlap`
  (params (OverlappedComponent :type "PrimitiveComponent Object Reference") (OtherActor :type "Actor Object Reference") (OtherComp :type "PrimitiveComponent Object Reference") (OtherBodyIndex :type Integer)))

(event `FriendFound`
  ;[0.7096 1 0.6208 0.2] FoundFriend
  (`ActorComponent.K2_DestroyComponent` (`self.Interact`))
  (bind _returnvalue (`KismetSystemLibrary.K2_SetTimerDelegate` (`|CreateDelegate` :!event `Position`) (`self.TimerDeltaTime`) true))
  (`self.Follow`))

(event `Follow`
  ;[1 0.5819 0.562 0.2] Follow
  (`|AIMoveTo` self (0.0 0.0 0.0) (`GameplayStatics.GetPlayerCharacter` 0) (`self.FollowDistance`)
    (:`OnSuccess`
      (`self.Follow`))))

(event `Position`
  (bind (_returnvalue_x _returnvalue_y _returnvalue_z) (`KismetMathLibrary.BreakVector` (`SceneComponent.K2_GetComponentLocation` (`self.Mesh`))))
  (bind _linearcolor (make `LinearColor` _returnvalue_x _returnvalue_y _returnvalue_z))
  ;[1 0.5156 0.5156 0.2] BakePosition
  (switch `/Game/Blueprints/Enumerators/E_FriendTag` (`self.FriendTag`)
    (:`NewEnumerator0`
      (`KismetMaterialLibrary.SetVectorParameterValue` "/Game/Materials/MPC/MPC_Player.MPC_Player" "Friend1Position" _linearcolor))
    (:`NewEnumerator1`
      (`KismetMaterialLibrary.SetVectorParameterValue` "/Game/Materials/MPC/MPC_Player.MPC_Player" "Friend2Position" _linearcolor))
    (:`NewEnumerator2`
      (`KismetMaterialLibrary.SetVectorParameterValue` "/Game/Materials/MPC/MPC_Player.MPC_Player" "Friend3Position" _linearcolor))
    (:`NewEnumerator3`
      (`KismetMaterialLibrary.SetVectorParameterValue` "/Game/Materials/MPC/MPC_Player.MPC_Player" "Friend4Position" _linearcolor))))

(fn `UserConstructionScript`
  (`SphereComponent.SetSphereRadius` (`self.Interact`) (`self.InteractArea`) true))