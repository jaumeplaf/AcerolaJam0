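; BP_LightBeam is a light beam actor whose three beam components appear in game only during the map's corrupted state.
; On BeginPlay it binds to the initial, corrupted and final state events of the first BP_MapManager found, then starts hidden.
; The state handlers toggle Hidden in Game on the beams.
; The construction script turns their visibility off, and BeginPlay restores it so Hidden in Game controls display.
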(event `init`
  (`SceneComponent.SetHiddenInGame` (`self.Beam01`) true true)
  (`SceneComponent.SetHiddenInGame` (`self.Beam03`) true true)
  (`SceneComponent.SetHiddenInGame` (`self.Beam02`) true true))

(event `corr`
  (`SceneComponent.SetHiddenInGame` (`self.Beam03`) false true)
  (`SceneComponent.SetHiddenInGame` (`self.Beam02`) false true)
  (`SceneComponent.SetHiddenInGame` (`self.Beam01`) false true))

(event `fina`
  (`SceneComponent.SetHiddenInGame` (`self.Beam03`) true true)
  (`SceneComponent.SetHiddenInGame` (`self.Beam02`) true true)
  (`SceneComponent.SetHiddenInGame` (`self.Beam01`) true true))

(event `self.ReceiveBeginPlay`
  (bind _beam03 (`self.Beam03`))
  (bind _outactors (`GameplayStatics.GetAllActorsOfClass` "/Game/Blueprints/BP_MapManager.BP_MapManager_C"))
  (bind _output (`|GetArrayItem` _outactors))
  (add `/Game/Blueprints/BP_MapManager.Map_Initial` _output (`|CreateDelegate` :!event `init`))
  (add `/Game/Blueprints/BP_MapManager.Map_Initial` _output (`|CreateDelegate` :!event `init`))
  (add `/Game/Blueprints/BP_MapManager.Map_Corrupted` _output (`|CreateDelegate` :!event `corr`))
  (add `/Game/Blueprints/BP_MapManager.Map_Final` _output (`|CreateDelegate` :!event `fina`))
  (`SceneComponent.SetHiddenInGame` _beam03 true true)
  (`SceneComponent.SetHiddenInGame` (`self.Beam02`) true true)
  (`SceneComponent.SetHiddenInGame` (`self.Beam01`) true true)
  (`SceneComponent.SetVisibility` _beam03 true false)
  (`SceneComponent.SetVisibility` (`self.Beam02`) true false)
  (`SceneComponent.SetVisibility` (`self.Beam01`) true false)
  (`self.init`))

(fn `UserConstructionScript`
  (`SceneComponent.SetVisibility` (`self.Beam03`) false false)
  (`SceneComponent.SetVisibility` (`self.Beam02`) false false)
  (`SceneComponent.SetVisibility` (`self.Beam01`) false false))