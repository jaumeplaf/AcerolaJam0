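; BP_Crater01 is a crater actor that reveals its waterfalls in response to dam events.
; On BeginPlay it finds every BP_Blockedway1 actor and binds its four dam events to each one.
; Each of the four dam events makes its matching waterfall component visible, without propagating visibility to children.
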(event `self.ReceiveBeginPlay`
  (bind _outactors (`GameplayStatics.GetAllActorsOfClass` "/Game/Blueprints/BP_Blockedway1.BP_Blockedway1_C"))
  (for _array_element _outactors
    (add `/Game/Blueprints/BP_Blockedway1.Dam01` _array_element (delegate `Dam01`))
    (add `/Game/Blueprints/BP_Blockedway1.Dam02` _array_element (delegate `Dam02`))
    (add `/Game/Blueprints/BP_Blockedway1.Dam03` _array_element (delegate `Dam03`))
    (add `/Game/Blueprints/BP_Blockedway1.Dam04` _array_element (delegate `Dam04`))))

(event `Dam01`
  (`SceneComponent.SetVisibility` (`self.WFall01`) true false))

(event `Dam02`
  (`SceneComponent.SetVisibility` (`self.WFall02`) true false))

(event `Dam03`
  (`SceneComponent.SetVisibility` (`self.WFall03`) true false))

(event `Dam04`
  (`SceneComponent.SetVisibility` (`self.WFall04`) true false))

(fn `UserConstructionScript`)