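; BP_Rocks is a rock actor that reacts to the map's Initial, Corrupted and Final states through events bound on BP_MapManager.
; Initial stops movement and records the starting height, with physics disabled at BeginPlay and mass scaled by actor size.
; Corrupted sets random spin and starts a looping timer that raises the rock at randomized speed, wrapping at MaxZ.
; Final stops timer and spin, then enables physics and gravity.
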(event `Initial`
  (bind (_returnvalue_x _returnvalue_y _returnvalue_z) (`KismetMathLibrary.BreakVector` (`SceneComponent.K2_GetComponentLocation` (`self.DefaultSceneRoot`))))
  (`KismetSystemLibrary.K2_ClearAndInvalidateTimerHandle` (stale `Corr` _returnvalue))
  (set `self.initial Z` _returnvalue_z))

(event `self.ReceiveBeginPlay`
  (bind _rock01 (`self.Rock01`))
  (bind _relativescale3d_x (`KismetMathLibrary.BreakVector` (`SceneComponent.RelativeScale3D` (`self.DefaultSceneRoot`))))
  (bind _outactors (`GameplayStatics.GetAllActorsOfClass` "/Game/Blueprints/BP_MapManager.BP_MapManager_C"))
  (bind _output (`|GetArrayItem` _outactors))
  (add `/Game/Blueprints/BP_MapManager.Map_Initial` _output (`|CreateDelegate` :!event `Initial`))
  (add `/Game/Blueprints/BP_MapManager.Map_Initial` _output (`|CreateDelegate` :!event `Initial`))
  (add `/Game/Blueprints/BP_MapManager.Map_Corrupted` _output (`|CreateDelegate` :!event `Corr`))
  (add `/Game/Blueprints/BP_MapManager.Map_Final` _output (`|CreateDelegate` :!event `Final`))
  (`PrimitiveComponent.SetSimulatePhysics` _rock01 false)
  (`PrimitiveComponent.SetMassScale` _rock01 "None" (* _relativescale3d_x 1000.0))
  (`self.Initial`))

(event `Corr`
  (set `RotatingMovementComponent.RotationRate` (`KismetMathLibrary.MakeRotator` (* (`KismetMathLibrary.RandomFloat`) 180.0) (* (`KismetMathLibrary.RandomFloat`) 180.0) (* (`KismetMathLibrary.RandomFloat`) 180.0)) (`self.RotatingMovement`))
  (bind _returnvalue (`KismetSystemLibrary.K2_SetTimerDelegate` (`|CreateDelegate` :!event `Move`) (`self.DeltaTime`) true))
  (goto _label :!via `Reset`))

(event `Final`
  (`KismetSystemLibrary.K2_ClearAndInvalidateTimerHandle` (stale `Corr` _returnvalue))
  (`PrimitiveComponent.SetSimulatePhysics` (`self.Rock01`) true)
  (`PrimitiveComponent.SetEnableGravity` (`self.Rock01`) true)
  (set `RotatingMovementComponent.RotationRate` (`KismetMathLibrary.MakeRotator` 0.0) (`self.RotatingMovement`)))

(event `Move`
  (bind (_returnvalue_x _returnvalue_y _returnvalue_z) (`KismetMathLibrary.BreakVector` (`SceneComponent.K2_GetComponentLocation` (`self.DefaultSceneRoot`))))
  (`|ExecutionSequence`
    (:`then_0`
      (`/Engine/EditorBlueprintResources/StandardMacros.DoOnce` false :!label _label
        (:`Completed`
          (`KismetSystemLibrary.Delay` (* (`KismetMathLibrary.RandomFloat`) 5.0)))))
    (:`then_1`
      (if (>= (`self.NewZ`) (`self.Max Z`))
        (bind _output_get (set `self.NewZ` (`self.initial Z`)))
        (`SceneComponent.K2_SetWorldLocation` (`self.DefaultSceneRoot`) (`KismetMathLibrary.MakeVector` _returnvalue_x _returnvalue_y _output_get) false false)
        (else
          (bind _output_get_2 (set `self.NewZ` (+ _returnvalue_z (* (`self.DeltaTime`) (* (`self.SpeedMult`) (+ (`KismetMathLibrary.RandomFloat`) 1.0))))))
          (`SceneComponent.K2_SetWorldLocation` (`self.DefaultSceneRoot`) (`KismetMathLibrary.MakeVector` _returnvalue_x _returnvalue_y _output_get_2) false false))))))

(event `self.ReceiveTick`
  (params (DeltaSeconds :type "Float (single-precision)")))

(fn `UserConstructionScript`)