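; BP_MapManager switches the map between Initial, Corrupted and Final states.
; BeginPlay binds map-state dispatchers and the little-guy character's change-map event, then starts Initial; a debug event cycles states.
; Initial and Corrupted toggle "Corrupted"-tagged actors' visibility and collision, the landscape Material Parameter Collection, and inversely the proxy floor's collision.
; The Final handler is empty.
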(event `Initialize`
  (bind _outactors (`GameplayStatics.GetAllActorsWithTag` "Corrupted"))
  (for _array_element _outactors
    (`self.SetActorHiddenInGame` _array_element true)
    (`self.SetActorEnableCollision` _array_element false)
    (`KismetMaterialLibrary.SetScalarParameterValue` "/Game/Materials/MPC/MPC_Landscape.MPC_Landscape" "Corrupted")
    (bind _outactors_2 (`GameplayStatics.GetAllActorsOfClass` "/Game/Blueprints/BP_ProxyFloor.BP_ProxyFloor_C"))
    (bind _floorplane (`/Game/Blueprints/BP_ProxyFloor.FloorPlane` (`|GetArrayItem` _outactors_2)))
    (set `self.ProxyFloor` _floorplane)
    (`PrimitiveComponent.SetCollisionEnabled` _floorplane "QueryAndPhysics")))

(event `Corrupt`
  (bind _outactors (`GameplayStatics.GetAllActorsWithTag` "Corrupted"))
  (for _array_element _outactors
    (`self.SetActorHiddenInGame` _array_element false)
    (`self.SetActorEnableCollision` _array_element true)
    (`KismetMaterialLibrary.SetScalarParameterValue` "/Game/Materials/MPC/MPC_Landscape.MPC_Landscape" "Corrupted" 1.0)
    (`PrimitiveComponent.SetCollisionEnabled` (`self.ProxyFloor`) "NoCollision")))

(event `Finalize`)

(event `self.ReceiveBeginPlay`
  (bind _asbp_character_little_guy (cast `/Game/Blueprints/BP_Character_LittleGuy` (`GameplayStatics.GetPlayerCharacter` 0)))
  (bind _output_get (set `self.As BP Character Little Guy` _asbp_character_little_guy))
  (add `/Game/Blueprints/BP_Character_LittleGuy.ChangeMapEvent` _output_get (`|CreateDelegate` :!event `Change`))
  (add `self.Map_Initial` (`|CreateDelegate` :!event `Initialize`))
  (add `self.Map_Corrupted` (`|CreateDelegate` :!event `Corrupt`))
  (add `self.Map_Final` (`|CreateDelegate` :!event `Finalize`))
  (`self.Map_Initial`))

(event `Change`
  ;[0.4937 1 0.6909 0.2] Switch between maps (debug)
  (switch `/Game/Blueprints/E_MapState` (`self.MapState`)
    (:`NewEnumerator0`
      (`self.Map_Corrupted`)
      (set `self.MapState` "NewEnumerator1")
      (`KismetSystemLibrary.PrintString` "CORRUPTED"))
    (:`NewEnumerator1`
      (`self.Map_Final`)
      (set `self.MapState` "NewEnumerator2")
      (`KismetSystemLibrary.PrintString` "FINAL"))
    (:`NewEnumerator2`
      (`self.Map_Initial`)
      (set `self.MapState` "NewEnumerator0")
      (`KismetSystemLibrary.PrintString` "INITIAL"))))

(fn `UserConstructionScript`)