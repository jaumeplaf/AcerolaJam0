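; Blocked-way indicator actor whose Plane pops up when something overlaps its Sphere and retracts when the overlap ends.
; Begin overlap moves the Plane to SpawnOffset height, then the Appear timeline reveals it, scaling it and lerping it toward its original Z.
; End overlap plays the Disappear timeline to scale and lerp it back.
; With Debug on, the construction script draws a vertical line and applies InteractArea as the Sphere radius.
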(event `self.ReceiveBeginPlay`
  (bind _sphere (`self.Sphere`))
  (bind (_returnvalue_x _returnvalue_y _returnvalue_z) (`KismetMathLibrary.BreakVector` (`SceneComponent.K2_GetComponentLocation` (`self.Plane`))))
  (`TimelineComponent.SetPlayRate` (`self.Appear`) 2.0)
  (`TimelineComponent.SetPlayRate` (`self.Disappear`) 0.1)
  (set `self.OriginalZpos` _returnvalue_z)
  (add `PrimitiveComponent.OnComponentBeginOverlap` _sphere (delegate `OnComponentBeginOverlap_Event`))
  (add `PrimitiveComponent.OnComponentEndOverlap` _sphere (delegate `OnComponentEndOverlap_Event`))
  (add `PrimitiveComponent.OnComponentEndOverlap` (`self.Sphere`) (delegate `OnComponentEndOverlap_Event`)))

(event `OnComponentBeginOverlap_Event`
  (params (OverlappedComponent :type "PrimitiveComponent Object Reference") (OtherActor :type "Actor Object Reference") (OtherComp :type "PrimitiveComponent Object Reference") (OtherBodyIndex :type Integer) (bFromSweep :type Boolean) (SweepResult :type "HitResult Structure (by ref)"))
  (bind (_returnvalue_x _returnvalue_y _returnvalue_z) (`KismetMathLibrary.BreakVector` (`SceneComponent.K2_GetComponentLocation` (`self.Plane`))))
  (bind (_returnvalue_x_2 _returnvalue_y_2 _returnvalue_z_2) (`KismetMathLibrary.BreakVector` (`SceneComponent.K2_GetComponentLocation` (`self.Plane`))))
  (bind (_returnvalue_x_3 _returnvalue_y_3 _returnvalue_z_3) (`KismetMathLibrary.BreakVector` (`SceneComponent.K2_GetComponentLocation` (`self.Plane`))))
  (`|ExecutionSequence`
    (:`then_0`
      (`|ExecutionSequence`
        (:`then_0`
          (goto _label_2 :!via `Reset`))
        (:`then_1`
          (bind (_direction _disappearinterpolate) (`Timeline|Disappear` :!via `Stop` :!label _label)
            (:`Update`
              (`|ExecutionSequence`
                (:`then_0`
                  (`/Engine/EditorBlueprintResources/StandardMacros.DoOnce` false :!label _label_2
                    (:`Completed`
                      (`PrimitiveComponent.SetRenderCustomDepth` (`self.Plane`) false))))
                (:`then_1`
                  (bind _returnvalue (* _disappearinterpolate 3.0))
                  (`SceneComponent.SetRelativeScale3D` (`self.Plane`) (`KismetMathLibrary.MakeVector` _returnvalue _returnvalue _returnvalue))
                  (`SceneComponent.K2_SetWorldLocation` (`self.Plane`) (`KismetMathLibrary.MakeVector` _returnvalue_x_2 _returnvalue_y_2 (`KismetMathLibrary.Lerp` (`self.SpawnOffset`) _returnvalue_z_2 _disappearinterpolate)) false false))))
            (:`Finished`
              (goto _label_2 :!via `Reset`))))))
    (:`then_1`
      (`SceneComponent.K2_SetWorldLocation` (`self.Plane`) (`KismetMathLibrary.MakeVector` _returnvalue_x_3 _returnvalue_y_3 (`self.SpawnOffset`)) false false)
      (bind (_direction_2 _appearinterpolate) (`Timeline|Appear` :!via `PlayFromStart` :!label _label_3)
        (:`Update`
          (`|ExecutionSequence`
            (:`then_0`
              (`/Engine/EditorBlueprintResources/StandardMacros.DoOnce` false :!label _label_4
                (:`Completed`
                  (`SceneComponent.SetVisibility` (`self.Plane`) true false))))
            (:`then_1`
              (bind _returnvalue_2 (* _appearinterpolate 3.0))
              (`SceneComponent.SetRelativeScale3D` (`self.Plane`) (`KismetMathLibrary.MakeVector` _returnvalue_2 _returnvalue_2 _returnvalue_2))
              (`SceneComponent.K2_SetWorldLocation` (`self.Plane`) (`KismetMathLibrary.MakeVector` _returnvalue_x _returnvalue_y (`KismetMathLibrary.Lerp` _returnvalue_z (`self.OriginalZpos`) _appearinterpolate)) false false))))
        (:`Finished`
          (goto _label_4 :!via `Reset`))))))

(event `OnComponentEndOverlap_Event`
  (params (OverlappedComponent :type "PrimitiveComponent Object Reference") (OtherActor :type "Actor Object Reference") (OtherComp :type "PrimitiveComponent Object Reference") (OtherBodyIndex :type Integer))
  (`|ExecutionSequence`
    (:`then_0`
      (goto _label_3 :!via `Stop`))
    (:`then_1`
      (goto _label :!via `PlayFromStart`))))

(fn `UserConstructionScript`
  (bind (_returnvalue_x _returnvalue_y _returnvalue_z) (`KismetMathLibrary.BreakVector` (`self.K2_GetActorLocation` self)))
  (bind _returnvalue (/ (`self.DebugLineSize`) 2.0))
  ;[1 0.588 0.6079 0.2] VisualizeLine
  (if (`self.Debug`)
    (`KismetSystemLibrary.FlushPersistentDebugLines`)
    (`KismetSystemLibrary.DrawDebugLine` (`KismetMathLibrary.MakeVector` _returnvalue_x _returnvalue_y (- _returnvalue_z _returnvalue)) (`KismetMathLibrary.MakeVector` _returnvalue_x _returnvalue_y (+ _returnvalue_z _returnvalue)) (struct :`R` 1.0 :`A` 1.0) 3600.0 3.0)
    (`SphereComponent.SetSphereRadius` (`self.Sphere`) (`self.InteractArea`) true)
    (else
      (`KismetSystemLibrary.FlushPersistentDebugLines`))))